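; BP_P38 is a player-controlled plane pawn that flies forward continuously and fires rockets.
; Tick adds movement input along the actor's forward vector, scaled by delta time and MoveSpeed.
; Pitch and Roll axis inputs apply frame-rate-scaled local rotations, both using PitchSpeed.
; The Fire action spawns a BP_Rocket at the Arrow component, facing its forward vector, with the plane as owner and instigator.
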(event `self.ReceiveTick`
  (params (DeltaSeconds :type "Float (single-precision)"))
  (`self.MoveForward` DeltaSeconds))

(event `InputAction|Fire`
  (params (Key :type "Key Structure"))
  (:`Pressed`
    (`self.Fire`)))

(event `InputAxis|Pitch`
  (params (AxisValue :type "Float (single-precision)"))
  (`self.InputRotation` AxisValue true))

(event `InputAxis|Roll`
  (params (AxisValue :type "Float (single-precision)"))
  (`self.InputRotation` AxisValue))

(fn `Fire`
  (bind _arrow (`self.Arrow`))
  (bind (_returnvalue_x _returnvalue_y _returnvalue_z) (`KismetMathLibrary.BreakVector` (`SceneComponent.K2_GetComponentLocation` _arrow)))
  (`|SpawnActorFromClass` "/Game/Blueprints/BP_Rocket.BP_Rocket_C" (`KismetMathLibrary.MakeTransform` (`KismetMathLibrary.MakeVector` _returnvalue_x _returnvalue_y _returnvalue_z) (`KismetMathLibrary.Conv_VectorToRotator` (`SceneComponent.GetForwardVector` _arrow))) "AdjustIfPossibleButAlwaysSpawn" "MultiplyWithRoot" self self))

(fn `InputRotation`
  (params (AxisValue :type "Float (double-precision)") (bIsPitch :type Boolean))
  (bind _returnvalue (* AxisValue (`GameplayStatics.GetWorldDeltaSeconds`) (`self.PitchSpeed`)))
  (if bIsPitch
    (`self.K2_AddActorLocalRotation` (`KismetMathLibrary.MakeRotator` 0.0 _returnvalue))
    (else
      (`self.K2_AddActorLocalRotation` (`KismetMathLibrary.MakeRotator` _returnvalue)))))

(fn `MoveForward`
  (params (A :type "Float (double-precision)"))
  (`self.AddMovementInput` (`self.GetActorForwardVector`) (* A (`self.MoveSpeed`))))

(fn `UserConstructionScript`)