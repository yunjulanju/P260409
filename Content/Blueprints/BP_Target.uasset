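; BP_Target is a damageable actor whose destruction triggers game over.
; Its AnyDamage event subtracts incoming damage from HP, and at zero or below it destroys the actor, casts the current game mode to BP_GameMode and calls GameOver.
; A separate chain that would cache the game mode reference is unconnected and never runs.
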(event `self.ReceiveBeginPlay`)

(event `self.ReceiveAnyDamage`
  (params (Damage :type "Float (single-precision)") (DamageType :type "DamageType Object Reference") (InstigatedBy :type "Controller Object Reference") (DamageCauser :type "Actor Object Reference"))
  (bind _output_get (set `self.HP` (- (`self.HP`) Damage)))
  (if (<= _output_get 0.0)
    (`self.K2_DestroyActor`)
    (bind _asbp_game_mode (cast `/Game/Blueprints/BP_GameMode` (`GameplayStatics.GetGameMode`)))
    (`/Game/Blueprints/BP_GameMode.GameOver` _asbp_game_mode)))

(fn `UserConstructionScript`)