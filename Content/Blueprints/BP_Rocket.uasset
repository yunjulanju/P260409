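; BP_Rocket is a short-lived projectile that damages what it hits and self-destructs after a few seconds if it hits nothing.
; On overlap with any actor not tagged Player, it spawns a small Niagara explosion and sound, then applies fixed damage to that actor only before destroying itself.
; Damage is credited to the first player controller.
; The graphs contain no movement logic.
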(event `self.ReceiveBeginPlay`
  ; 수명
  (`self.SetLifeSpan` 3.0))

(event `self.ReceiveActorBeginOverlap`
  (params (OtherActor :type "Actor Object Reference"))
  (bind _returnvalue (`self.K2_GetActorLocation`))
  (if (not (`self.ActorHasTag` OtherActor "Player"))
    (`NiagaraFunctionLibrary.SpawnSystemAtLocation` "/Game/NiagaraExamples/FX_Explosions/NS_Explosion_Small.NS_Explosion_Small" _returnvalue (struct) (1.0 1.0 1.0) true true "AutoRelease")
    (`GameplayStatics.PlaySoundAtLocation` "/Game/Sound/MS_Explotion.MS_Explotion" _returnvalue (struct) 1.0 1.0 0.0 null null null null)
    ; 0보다 커야 데미지 처리가 됨.
    (`GameplayStatics.ApplyDamage` OtherActor 10.0 (`GameplayStatics.GetPlayerController` 0) self)
    (`self.K2_DestroyActor`)))

(fn `UserConstructionScript`)